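; InstructionStack tracks instructions in a Stack collection to detect when an instruction sequence is stuck.
; Add, Contains and Reset record, look up and clear the tracked instructions.
; IsStuck flags an instruction that is already on the stack and takes no time, printing a debug hint to consider a reset; repeats of timed instructions are not flagged.
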(fn `Add`
  (params (Instruction :type "/Game/Blueprints/Instructions/Instruction Object Reference (by ref)"))
  (`BlueprintSetLibrary.Set_Add` (`self.Stack`) Instruction))

(fn `Contains`
  (params (Instruction :type "/Game/Blueprints/Instructions/Instruction Object Reference (by ref)"))
  (returns (Found :type Boolean))
  (return (`BlueprintSetLibrary.Set_Contains` (`self.Stack`) Instruction)))

(fn `IsStuck`
  (params (Instruction :type "/Game/Blueprints/Instructions/Instruction Object Reference"))
  (returns (Result :type Boolean))
  (if (`self.Contains` Instruction)
    (if (`/Game/Blueprints/Instructions/Instruction.TakesTime` Instruction)
      (return false)
      (else
        (`GameUtils.PrintDebugString` null "Stuck, consider reset")
        (return true)))
    (else
      (return false))))

(fn `Reset`
  (`BlueprintSetLibrary.Set_Clear` (`self.Stack`)))
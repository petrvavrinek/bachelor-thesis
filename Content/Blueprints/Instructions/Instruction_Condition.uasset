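; Instruction_Condition is a branching job instruction that runs either a Then or an Else instruction buffer on the controlled pawn.
; StartJob picks the buffer through CanActivate, starts it, and completes itself when the buffer's completion delegate fires, or immediately with a debug message if it is null.
; OnCopy creates fresh empty buffers for both branches.
; CanActivate is a placeholder that always returns true, so only Then is ever chosen.
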(event `self.OnCopy`
  ;[1 1 1] Initialize empty buffers
  (`parent.OnCopy`)
  (bind _returnvalue (`|GenericCreateObject` "/Game/Blueprints/Instructions/Base/InstructionBuffer.InstructionBuffer_C"))
  (set `self.ThenOperation` _returnvalue)
  (bind _returnvalue_2 (`|GenericCreateObject` "/Game/Blueprints/Instructions/Base/InstructionBuffer.InstructionBuffer_C"))
  (set `self.ElseOperation` _returnvalue_2))

(event `ProcessInstruction`
  (params (InstructionBuffer :type "/Game/Blueprints/Instructions/Base/Instruction Object Reference") (Pawn :type "Pawn Object Reference"))
  ;[1 1 1] Process instruction no matter which one
  (add `self.OnCompletedDelegate` InstructionBuffer (delegate `OnInstructionCompleted`))
  (`self.StartJob` InstructionBuffer Pawn))

(event `OnInstructionCompleted`
  ;[1 1 1] Process instruction no matter which one
  (`/Engine/EditorBlueprintResources/StandardMacros.IsValid` (stale `ProcessInstruction` InstructionBuffer)
    (:`Is Valid`
      (remove `self.OnCompletedDelegate` (stale `ProcessInstruction` InstructionBuffer) (delegate `OnInstructionCompleted`)))
    (:`Is Not Valid`
      _))
  (`self.OnJobCompleted`))

(event `self.StartJob`
  (params (ControlledPawn :type "Pawn Object Reference"))
  (bind _canactivate (`self.CanActivate`))
  (bind _returnvalue (select `bool` _canactivate :`false` (`self.ElseOperation`) :`true` (`self.ThenOperation`) :!type "/Game/Blueprints/Instructions/Base/Instruction Object Reference"))
  ;[1 1 1] Run operations based on condition
  (`/Engine/EditorBlueprintResources/StandardMacros.IsValid` _returnvalue
    (:`Is Valid`
      (`self.ProcessInstruction` _returnvalue ControlledPawn))
    (:`Is Not Valid`
      (`GameUtils.PrintDebugString` null (`KismetMathLibrary.SelectString` "Then instruction is NULL" "Else instruction is NULL" _canactivate))
      (`self.OnJobCompleted`))))

(fn `CanActivate`
  (returns (CanActivate :type Boolean))
  ;[1 1 1] TODO: Process condition
  (return true))
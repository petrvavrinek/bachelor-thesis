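; Instruction that holds an editable queue of child instructions and runs them in order as a single job for a controlled pawn.
; StartJob copies the queue into a working job queue, then starts each entry in turn, advancing through its completion callback until empty.
; An executor interrupt halts the chain, while a child exception, invalid executor or stuck call stack completes the job, passing an exception where one applies.
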(event `InsertInstructionAtIndex`
  (params (Instruction :type "/Game/Blueprints/Instructions/Instruction Object Reference (by ref)") (Index :type Integer))
  ;[1 1 1] Overriden StartJob for arrays
  (`KismetArrayLibrary.Array_Insert` (`self.InstructionQueue`) Instruction Index))

(event `ClearQueue`
  ;[1 1 1] Overriden StartJob for arrays
  ;;[1 1 1] Clear queue
  (`KismetArrayLibrary.Array_Clear` (`self.InstructionQueue`)))

(event `StartJobSkipArrayCopy`
  (params (Pawn :type "Pawn Object Reference") (Executor :type "/Game/Blueprints/Instructions/InstructionExecutor Object Reference"))
  (bind _instrucutionjobqueue (`self.InstrucutionJobQueue`))
  (bind _output (`|GetArrayItem` _instrucutionjobqueue))
  ;[1 1 1] Overriden StartJob for arrays
  (`/Engine/EditorBlueprintResources/StandardMacros.IsValid` Executor
    (:`Is Valid`
      (if (`/Game/Blueprints/Instructions/InstructionExecutor.ShoudInterrupt` Executor)
        _
        (elif (`KismetArrayLibrary.Array_IsEmpty` _instrucutionjobqueue)
          (`self.CompleteJob` null Executor Pawn)
          (elif (`/Game/Blueprints/Instructions/InstructionStack.IsStuck` (`/Game/Blueprints/Instructions/InstructionExecutor.InstructionCallStack` Executor) _output)
            (bind _returnvalue (`|GenericCreateObject` "/Game/Blueprints/Instructions/InstructionExceptions/InstructionException_CallExceeded.InstructionException_CallExceeded_C"))
            (`self.CompleteJob` _returnvalue Executor Pawn)
            (else
              (add `self.OnCompleted` _output (delegate `OnCompletedInstruction`))
              (`self.StartJob` _output Pawn Executor))))))
    (:`Is Not Valid`
      (bind _returnvalue_2 (`|GenericCreateObject` "/Game/Blueprints/Instructions/InstructionExceptions/InstructionException_InvalidExecutor.InstructionException_InvalidExecutor_C"))
      (`self.CompleteJob` _returnvalue_2 null Pawn))))

(event `OnCompletedInstruction` :!signature `self.OnCompleted`
  (params (Exception :type "/Game/Blueprints/Instructions/InstructionException Object Reference") (Executor :type "/Game/Blueprints/Instructions/InstructionExecutor Object Reference") (ControlledPawn :type "Pawn Object Reference"))
  ;[1 1 1] Overriden StartJob for arrays
  (remove `self.OnCompleted` (`|GetArrayItem` (`self.InstrucutionJobQueue`)) (delegate `OnCompletedInstruction`))
  (`/Engine/EditorBlueprintResources/StandardMacros.IsValid` Exception
    (:`Is Valid`
      (`self.OnJobCompleted` Exception Executor ControlledPawn))
    (:`Is Not Valid`
      (`KismetArrayLibrary.Array_Remove` (`self.InstrucutionJobQueue`))
      (`self.StartJobSkipArrayCopy` ControlledPawn Executor))))

(event `self.StartJob`
  (params (ControlledPawn :type "Pawn Object Reference") (Executor :type "/Game/Blueprints/Instructions/InstructionExecutor Object Reference"))
  ;[1 1 1] Overriden StartJob for arrays
  (`parent.StartJob` ControlledPawn Executor)
  (`self.CopyQueue` (`self.InstructionQueue`) (`self.InstrucutionJobQueue`))
  (`self.StartJobSkipArrayCopy` ControlledPawn Executor))

(fn `CopyQueue`
  (params (From :type "Array of /Game/Blueprints/Instructions/Instruction Object Reference") (To :type "Array of /Game/Blueprints/Instructions/Instruction Object Reference"))
  (`KismetArrayLibrary.Array_Clear` To)
  (`KismetArrayLibrary.Array_Resize` To (`KismetArrayLibrary.Array_Length` From))
  (for _index (range (+ (`KismetArrayLibrary.Array_LastIndex` From) 1))
    (`KismetArrayLibrary.Array_Set` To _index (`|GetArrayItem` From _index)))
  (return))

(fn `GetCurrentJob`
  (returns (Output :type "/Game/Blueprints/Instructions/Instruction Object Reference"))
  (return (`|GetArrayItem` (`self.InstructionQueue`))))

(fn `RemoveInstructionAtIndex`
  (params (Index :type Integer))
  (`KismetArrayLibrary.Array_Remove` (`self.InstructionQueue`) Index))

(fn `SetIndexNewIndex`
  (params (Index :type Integer) (NewIndex :type Integer))
  (locals (ElementValue :type "/Game/Blueprints/Instructions/Instruction Object Reference"))
  (bind _outarray (`/Game/Blueprints/Macros/ArrayHelper.MoveIndex` (`self.InstructionQueue`) Index NewIndex)
    (:`Return`
      (set `self.InstructionQueue` _outarray))))
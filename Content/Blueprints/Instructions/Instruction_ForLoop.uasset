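; Loop instruction that repeats its queue of child instructions on a controlled pawn, built on a parent instruction class.
; StartJob stores the pawn and runs the parent job, or completes at once if the queue is empty.
; On each completion, ConditionCheck compares a counter to a hard-coded limit, then either restarts the parent job or finishes and resets the counter.
; Debug prints trace each check and restart.
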(event `/Game/Blueprints/Instructions/Base/Instruction.OnJobCompleted`
  (if (`self.ConditionCheck`)
    (`parent.StartJob` (`self.ControlledPawn`))
    (`/Engine/EditorBlueprintResources/StandardMacros.IncrementInt` (`self.Counter`)
      (:`  `
        (`GameUtils.PrintDebugString` null "Start")))
    (else
      (`parent.OnJobCompleted`)
      (set `self.Counter` 0))))

(event `CustomEvent`)

(event `self.StartJob`
  (params (ControlledPawn :type "Pawn Object Reference"))
  (bind _output_get (set `self.ControlledPawn` ControlledPawn))
  (if (`KismetArrayLibrary.Array_IsEmpty` (`self.InstructionQueue`))
    (`parent.OnJobCompleted`)
    (else
      (`parent.StartJob` _output_get))))

(fn `ConditionCheck`
  (returns (ReturnValue :type Boolean))
  (bind _counter (`self.Counter`))
  (`GameUtils.PrintDebugString` null (`KismetStringLibrary.BuildString_Int` "Check no. " "" _counter) (struct :`R` 1.0 :`A` 1.0))
  (return (< _counter 3)))
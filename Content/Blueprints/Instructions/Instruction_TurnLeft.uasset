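; Instruction job that makes the player robot turn left, run on the controlled pawn.
; On start it casts the pawn to BP_PlayerRobot, binds to its instruction-completed event and calls TurnLeft, passing itself as the instruction.
; When the completed instruction matches itself, it unbinds and reports job completion; otherwise it prints an error.
; The completion handler is named OnMoveForwardCompleted despite handling the turn.
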(event `self.StartJob`
  (params (ControlledPawn :type "Pawn Object Reference"))
  (`self.OnJobStarted`)
  (bind _asbp_player_robot (cast `/Game/Blueprints/Pawns/BP_PlayerRobot` ControlledPawn))
  (add `/Game/Blueprints/Pawns/BP_PlayerRobot.OnInstructionCompleted` _asbp_player_robot (delegate `OnMoveForwardCompleted`))
  (`/Game/Blueprints/Pawns/BP_PlayerRobot.TurnLeft` _asbp_player_robot self))

(event `OnMoveForwardCompleted`
  (params (Instruction :type "/Game/Blueprints/Instructions/Base/Instruction Object Reference"))
  (if (== Instruction self)
    (remove `/Game/Blueprints/Pawns/BP_PlayerRobot.OnInstructionCompleted` (stale `self.StartJob` _asbp_player_robot) (delegate `OnMoveForwardCompleted`))
    (`self.OnJobCompleted`)
    (else
      (`KismetSystemLibrary.PrintString` (stale `self.StartJob` _asbp_player_robot) "Wrong completed instruction"))))
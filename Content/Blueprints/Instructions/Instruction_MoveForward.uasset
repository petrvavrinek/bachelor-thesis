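; Robot instruction that makes the controlled pawn move forward as a job.
; On start it signals started, casts the pawn to Robot, calls MoveForward with itself, then binds to the robot's instruction-completed event.
; The completion handler signals completed only when the reported instruction is itself, and otherwise prints a wrong-instruction message.
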(event `self.StartJob`
  (params (ControlledPawn :type "Pawn Object Reference"))
  (`self.OnStarted`)
  (bind _asrobot (cast `/Game/Blueprints/Robot` ControlledPawn))
  (`/Game/Blueprints/Robot.MoveForward` _asrobot self)
  (add `/Game/Blueprints/Robot.OnInstructionCompleted` _asrobot (delegate `OnMoveForwardCompleted`)))

(event `OnMoveForwardCompleted`
  (params (Instruction :type "/Game/Blueprints/Instructions/Base/Instruction Object Reference"))
  (if (== Instruction self)
    (`self.OnCompleted`)
    (else
      (`KismetSystemLibrary.PrintString` (stale `self.StartJob` _asrobot) "Wrong completed instruction"))))
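; Base Instruction object that represents a job for a controlled pawn, tracking whether it is in progress.
; StartJob by default only raises OnJobStarted to set the InProgress flag.
; CompleteJob routes to OnJobCompleted, which clears the flag and broadcasts the OnCompleted dispatcher with the pawn.
; OnCopy, meant to be called when the object is copied, unbinds all OnCompleted listeners.
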(event `OnCopy`
  ;[1 1 1] This needs to be called on copy
  (clear `self.OnCompleted`))

(event `OnJobCompleted`
  (params (ControlledPawn :type "Pawn Object Reference"))
  ;[1 1 1] This event must be trigged manually on object init
  (set `self.InProgress` false)
  (`self.OnCompleted` ControlledPawn))

(event `OnJobStarted`
  ;[1 1 1] This event must be trigged manually on object init
  (set `self.InProgress` true))

(event `StartJob`
  (params (ControlledPawn :type "Pawn Object Reference"))
  ;[1 1 1] Default behaviour
  (`self.OnJobStarted`))

(event `CompleteJob`
  (params (ControlledPawn :type "Pawn Object Reference"))
  ;[1 1 1] Default behaviour
  (`self.OnJobCompleted` ControlledPawn))

(fn `IsInProgress`
  (returns (InProgress :type Boolean))
  (return (`self.InProgress`)))
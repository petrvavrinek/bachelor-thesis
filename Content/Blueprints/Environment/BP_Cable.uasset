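; Environment cable actor that turns a hand-placed spline into a right-angled, grid-aligned run of instanced meshes.
; The construction script snaps spline points to GridSize and inserts corner points between them, stepping along Y, then Z, then X.
; Each resulting segment gets one instance at its midpoint, aimed at the next point, shifted by AdditionalOffset in segment space and stretched along X to fit.
; The event graph has no active logic.
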(fn `ClampVector`
  (params (Vector :type "Vector Structure") (Min :type "Float (double-precision)") (Max :type "Float (double-precision)"))
  (returns (OutVector :type "Vector Structure"))
  (return (`KismetMathLibrary.MakeVector` (`KismetMathLibrary.FClamp` (.x Vector) Min Max) (`KismetMathLibrary.FClamp` (.y Vector) Min Max) (`KismetMathLibrary.FClamp` (.z Vector) Min Max))))

(fn `Get Ideal Points Between Two Points`
  (params (Source :type "Vector Structure") (Goal :type "Vector Structure"))
  (returns (Points :type "Array of Vector Structure"))
  (locals (OutPoints :type "Array of Vector Structure"))
  (bind _x (.x Source))
  (bind _y (.y Goal))
  (bind _snapped (`self.SnapVectorGrid` Source))
  (bind _snapped_2 (`self.SnapVectorGrid` (`KismetMathLibrary.MakeVector` _x _y (.z Source))))
  (bind _snapped_3 (`self.SnapVectorGrid` (`KismetMathLibrary.MakeVector` _x _y (.z Goal))))
  (`|ExecutionSequence`
    (:`then_0`
      (if (not (== _snapped _snapped_2 :`ErrorTolerance` 1.0))
        (`KismetArrayLibrary.Array_Add` (`local.OutPoints`) _snapped_2)))
    (:`then_1`
      (if (not (== _snapped _snapped_3 :`ErrorTolerance` 1.0))
        (`KismetArrayLibrary.Array_Add` (`local.OutPoints`) _snapped_3)))
    (:`then_2`
      (return (`local.OutPoints`)))))

(fn `SnapVectorGrid`
  (params (Location :type "Vector Structure"))
  (returns (Snapped :type "Vector Structure"))
  (return (`KismetMathLibrary.Vector_SnappedToGrid` Location (`self.GridSize`))))

(fn `TruncateRotation`
  (params (InRotation :type "Rotator Structure"))
  (returns (OutRotation :type "Rotator Structure"))
  (return (`KismetMathLibrary.MakeRotator` 0.0 0.0 InRotation_Yaw)))

(fn `UserConstructionScript`
  (locals (CurrentSplineMeshComponent :type "SplineMeshComponent Object Reference") (LastLocation :type "Vector Structure") (Points :type "Array of Vector Structure"))
  (bind _spline (`self.Spline`))
  (bind _points (`local.Points`))
  (for _index (range (+ (`SplineComponent.GetNumberOfSplinePoints` _spline) 1))
    (bind _snapped (`self.SnapVectorGrid` (`SplineComponent.GetLocationAtSplinePoint` _spline _index "Local")))
    (`KismetArrayLibrary.Array_Add` (`local.Points`) _snapped)
    (bind _points_2 (`self.Get Ideal Points Between Two Points` _snapped (`self.SnapVectorGrid` (`SplineComponent.GetLocationAtSplinePoint` _spline (+ _index 1) "Local"))))
    (for _array_element _points_2
      (`KismetArrayLibrary.Array_Add` (`local.Points`) _array_element)))
  (for _index_2 (range (`KismetArrayLibrary.Array_LastIndex` (`local.Points`)))
    (bind _output (`|GetArrayItem` _points _index_2))
    (bind _output_2 (`|GetArrayItem` _points (+ _index_2 1)))
    (bind _returnvalue (`KismetMathLibrary.FindLookAtRotation` _output _output_2))
    (bind _returnvalue_2 (`KismetMathLibrary.Vector_Distance` _output _output_2))
    (`InstancedStaticMeshComponent.AddInstance` (`self.InstancedStaticMesh`) (`KismetMathLibrary.MakeTransform` (`KismetMathLibrary.GreaterGreater_VectorRotator` (+ (+ (`KismetMathLibrary.LessLess_VectorRotator` _output _returnvalue) (`self.AdditionalOffset`)) (`KismetMathLibrary.MakeVector` (/ _returnvalue_2 2.0))) _returnvalue) _returnvalue (`KismetMathLibrary.MakeVector` (/ _returnvalue_2 (`self.GridSize`)) 1.0 1.0)) false)))
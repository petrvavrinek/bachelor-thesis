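; BP_LevitatingMesh is an environment actor that makes a configurable mesh float back and forth while spinning.
; The construction script applies the chosen mesh and scale to the StaticMesh component.
; Each Tick feeds accumulated time into a sine wave, remapped between min and max offsets along LocationDirection to set relative location.
; It also adds a frame-rate-independent local rotation from RotationSpeed and RotationDirection.
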(event `self.ReceiveTick`
  (params (DeltaSeconds :type "Float (single-precision)"))
  (bind (_returnvalue_x _returnvalue_y _returnvalue_z) (`KismetMathLibrary.BreakVector` (* (* DeltaSeconds (`self.RotationSpeed`)) (`self.RotationDirection`))))
  (bind _output_get (set `self.AccumulatedDelta` (+ DeltaSeconds (`self.AccumulatedDelta`))))
  ;[1 1 1] Z Location set
  (`|ExecutionSequence`
    (:`then_0`
      (`SceneComponent.K2_SetRelativeLocation` (`self.StaticMesh`) (* (`KismetMathLibrary.MapRangeClamped` (* (+ (`KismetMathLibrary.Sin` (* _output_get (`self.LocationSpeed`))) 1.0) 0.5) 0.0 1.0 (`self.MinLocation`) (`self.MaxLocation`)) (`self.LocationDirection`)) false false))
    (:`then_1`
      ;[1 1 1] Rotation
      (`SceneComponent.K2_AddLocalRotation` (`self.StaticMesh`) (`KismetMathLibrary.MakeRotator` _returnvalue_x _returnvalue_y _returnvalue_z) false false))))

(fn `UserConstructionScript`
  (bind _staticmesh (`self.StaticMesh`))
  (`StaticMeshComponent.SetStaticMesh` _staticmesh (`self.Mesh`))
  (`SceneComponent.SetRelativeScale3D` _staticmesh (`self.MeshScale`)))
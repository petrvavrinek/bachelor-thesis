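; Robot pawn that carries out movement instructions, spawning its default AI controller on BeginPlay.
; MoveForward uses AIMoveTo to step a fixed distance along the forward vector, while TurnLeft uses a timeline to decrease yaw from its starting value.
; Each action passes its Instruction to OnInstructionCompleted when it finishes, though a failed move reports nothing.
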(event `self.ReceiveBeginPlay`
  (`self.SpawnDefaultController`))

(event `MoveForward`
  (params (Instruction :type "/Game/Blueprints/Instructions/Base/Instruction Object Reference"))
  (`|AIMoveTo` self (+ (* (`self.GetActorForwardVector`) (100.0 100.0 100.0)) (`self.K2_GetActorLocation`)) null 0.001
    (:`OnSuccess`
      (`self.OnInstructionCompleted` Instruction))))

(event `TurnLeft`
  (params (Instruction :type "/Game/Blueprints/Instructions/Base/Instruction Object Reference"))
  (bind (_returnvalue_roll _returnvalue_pitch _returnvalue_yaw) (`KismetMathLibrary.BreakRotator` (`self.K2_GetActorRotation`)))
  (set `self.StartRotationZ` _returnvalue_yaw)
  (bind (_direction _rotationz) (`Timeline|TurnLeftTimeline` :!via `PlayFromStart`)
    (:`Update`
      (`self.K2_SetActorRotation` (`KismetMathLibrary.MakeRotator` _returnvalue_roll _returnvalue_pitch (- (`self.StartRotationZ`) _rotationz))))
    (:`Finished`
      (`self.OnInstructionCompleted` Instruction))))

(fn `UserConstructionScript`)
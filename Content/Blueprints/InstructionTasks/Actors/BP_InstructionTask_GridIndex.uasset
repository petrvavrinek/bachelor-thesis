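; BP_InstructionTask_GridIndex is a placeable actor that supplies a grid-index instruction task based on where it sits.
; GetInstructionTasks finds the grid index closest to the actor through the grid manager and constructs an InstructionTask_GridIndex targeting it.
; If that index has a location, the actor teleports to snap onto it and returns the task; otherwise no task is returned.
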(fn `GetInstructionTasks`
  (returns (InstructionTasks :type "Array of /Game/Blueprints/InstructionTasks/InstructionTask Object Reference"))
  (bind _output (`/Game/Blueprints/Functions/GridFunctions.GetGridManager`))
  (bind _outputpin (`/Game/Blueprints/Grid/BP_Grid_Manager.GetClosestIndex` _output (`self.K2_GetActorLocation`)))
  (bind (_location _found) (`/Game/Blueprints/Grid/BP_Grid_Manager.GetIndexLocation` _output _outputpin))
  (`/Engine/EditorBlueprintResources/StandardMacros.IsValid` _output
    (:`Is Valid`
      (bind _returnvalue (`|GenericCreateObject` "/Game/Blueprints/InstructionTasks/InstructionTasks/InstructionTask_GridIndex.InstructionTask_GridIndex_C" _output _outputpin))
      (if _found
        (`self.K2_SetActorLocation` _location false true)
        (return (`|MakeArray` _returnvalue :!type "/Game/Blueprints/InstructionTasks/InstructionTask Object Reference"))))
    (:`Is Not Valid`
      (return))))

(fn `UserConstructionScript`)
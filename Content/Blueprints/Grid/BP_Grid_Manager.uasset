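; Grid manager that builds and serves a map of valid grid indices to world locations, with lookup helpers for validity, location and closest index.
; Shortly after BeginPlay, or through a Reset toggle in the construction script, it gathers valid indices from every BP_Grid_Bounds, ignoring Pawns.
; Each bounds' grid renderer draws its indices, which are merged into the shared map.
; Other helpers convert locations to indices by grid size and expand volume bounds into index points.
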(event `GetGridIndicesAndRender`
  (bind _outactors (`GameplayStatics.GetAllActorsOfClass` "/Script/Engine.Pawn"))
  (`self.RenderIndices` _outactors))

(event `self.ReceiveBeginPlay`
  (`KismetSystemLibrary.Delay` 0.2)
  (`self.GetGridIndicesAndRender`))

(fn `GetClosestIndex`
  (params (Index :type "Vector Structure"))
  (returns (OutputPin :type "IntPoint Structure"))
  (locals (Closest :type "IntPoint Structure") (ClosestDistance :type "Float (double-precision)" :default 999999999.0))
  (bind _gridindices (`self.GridIndices`))
  (bind _keys (`BlueprintMapLibrary.Map_Keys` _gridindices))
  (for _array_element _keys
    (bind (_value _returnvalue) (`BlueprintMapLibrary.Map_Find` _gridindices _array_element))
    (if _returnvalue
      (bind _returnvalue_2 (`KismetMathLibrary.Vector_Distance` _value Index))
      (if (< _returnvalue_2 (`local.ClosestDistance`))
        (set `local.ClosestDistance` _returnvalue_2)
        (set `local.Closest` _array_element))))
  (return (`local.Closest`)))

(fn `GetIndexLocation`
  (params (Index :type "IntPoint Structure"))
  (returns (Location :type "Vector Structure") (Found :type Boolean))
  (bind (_value _returnvalue) (`BlueprintMapLibrary.Map_Find` (`self.GridIndices`) Index))
  (return _value _returnvalue))

(fn `GetLocationIndex`
  (params (Location :type "Vector Structure"))
  (returns (Index :type "IntPoint Structure"))
  (bind _gridsize (`self.GridSize`))
  (return (make `IntPoint` (`KismetMathLibrary.FFloor` (/ (.x Location) _gridsize)) (`KismetMathLibrary.FFloor` (/ (.y Location) _gridsize)))))

(fn `GetNavMeshIndices`
  (params (NavVolumes :type "Array of NavMeshBoundsVolume Object Reference"))
  (returns (FoundPoints :type "Set of IntPoint Structure"))
  (locals (Points :type "Set of IntPoint Structure") (Origin :type "Vector Structure") (OriginIndex :type "IntPoint Structure"))
  (for _array_element NavVolumes
    (bind (_origin _boxextent) (`self.GetActorBounds` _array_element false false))
    (set `local.OriginIndex` (`self.GetLocationIndex` _origin))
    (bind (_index_x _index_y) (break `IntPoint` (`self.GetLocationIndex` _boxextent)))
    (for _index (range (* _index_x -1) (+ _index_x 1))
      (for _index_2 (range (* _index_y -1) (+ _index_y 1))
        (`BlueprintSetLibrary.Set_Add` (`local.Points`) (+ (make `IntPoint` _index _index_2) (`local.OriginIndex`))))))
  (return (`local.Points`)))

(fn `IsIndexValid`
  (params (Index :type "IntPoint Structure"))
  (returns (NewParam :type Boolean))
  (return (`BlueprintMapLibrary.Map_Contains` (`self.GridIndices`) Index)))

(fn `RenderIndices`
  (params (IgnoredActors :type "Array of Actor Object Reference"))
  (locals (Indices :type "Map of IntPoint Structure to Vector Structure"))
  (`BlueprintMapLibrary.Map_Clear` (`self.GridIndices`))
  (bind _outactors (`GameplayStatics.GetAllActorsOfClass` "/Game/Blueprints/Grid/BP_Grid_Bounds.BP_Grid_Bounds_C"))
  (for _array_element _outactors
    (bind _result (`/Game/Blueprints/Grid/BP_Grid_Bounds.GetValidIndices` _array_element self IgnoredActors))
    (`|ExecutionSequence`
      (:`then_0`
        (bind _gridrenderer (`/Game/Blueprints/Grid/BP_Grid_Bounds.GetGridRenderer` _array_element))
        (`/Engine/EditorBlueprintResources/StandardMacros.IsValid` _gridrenderer
          (:`Is Valid`
            (`/Game/Blueprints/Grid/BP_Grid_Renderer.RenderGrid` _gridrenderer _result))))
      (:`then_1`
        (bind _keys (`BlueprintMapLibrary.Map_Keys` _result))
        (for _array_element_2 _keys
          (`BlueprintMapLibrary.Map_Add` (`self.GridIndices`) _array_element_2 (`BlueprintMapLibrary.Map_Find` _result _array_element_2))))))
  (return))

(fn `UserConstructionScript`
  (locals (Origin :type "Vector Structure" :default (0.0 0.0 0.0)))
  ;[1 1 1] Reset function
  (if (`self.Reset`)
    (set `self.Reset` false)
    (`self.GetGridIndicesAndRender`)))
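; BP_Grid_Renderer draws a grid as instances of a hierarchical instanced static mesh.
; RenderGrid clears existing instances, then adds one world-space instance per location value in the supplied Indices map, applying a shared offset and scale with zero rotation.
; The construction script uses a self-resetting Reset flag as an editor toggle to clear all instances.
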(event `RenderGrid`
  (params (Indices :type "Map of IntPoint Structure to Vector Structure"))
  (`InstancedStaticMeshComponent.ClearInstances` (`self.HierarchicalInstancedStaticMesh`))
  (bind _values (`BlueprintMapLibrary.Map_Values` Indices))
  (for _array_element _values
    (`InstancedStaticMeshComponent.AddInstance` (`self.HierarchicalInstancedStaticMesh`) (`KismetMathLibrary.MakeTransform` (+ _array_element (`self.Offset`)) (struct) (`self.Scale`)) true)))

(fn `UserConstructionScript`
  (if (`self.Reset`)
    (set `self.Reset` false)
    (`InstancedStaticMeshComponent.ClearInstances` (`self.HierarchicalInstancedStaticMesh`))))
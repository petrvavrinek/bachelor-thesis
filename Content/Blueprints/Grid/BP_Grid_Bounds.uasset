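; Grid bounds Blueprint whose box defines a region of grid cells and finds which of them have a surface.
; GetCollisionBoxIndices uses the GridManager to turn the box's location and extent into a range of 2D indices.
; GetValidIndices line-traces vertically through each cell around Z zero on Visibility, mapping hit indices to hit locations.
; GetGridRenderer returns a cached or found renderer, otherwise spawns one without caching it.
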(fn `GetCollisionBoxIndices`
  (params (GridManager :type "/Game/Blueprints/Grid/BP_Grid_Manager Object Reference"))
  (returns (Indices :type "Array of IntPoint Structure"))
  (locals (BoxIndices :type "Array of IntPoint Structure") (OriginIndex :type "IntPoint Structure"))
  (bind _box (`self.Box`))
  (bind (_index_x _index_y) (break `IntPoint` (`/Game/Blueprints/Grid/BP_Grid_Manager.GetLocationIndex` GridManager (`BoxComponent.BoxExtent` _box))))
  (set `local.OriginIndex` (`/Game/Blueprints/Grid/BP_Grid_Manager.GetLocationIndex` GridManager (`SceneComponent.K2_GetComponentLocation` _box)))
  (for _index (range (* _index_x -1) (+ _index_x 1))
    (for _index_2 (range (* _index_y -1) (+ _index_y 1))
      (`KismetArrayLibrary.Array_Add` (`local.BoxIndices`) (+ (make `IntPoint` _index _index_2) (`local.OriginIndex`)))))
  (return (`local.BoxIndices`)))

(fn `GetGridRenderer`
  (returns (GridRenderer :type "/Game/Blueprints/Grid/BP_Grid_Renderer Object Reference"))
  (bind _gridrendererclass (`self.GridRendererClass`))
  (`/Engine/EditorBlueprintResources/StandardMacros.IsValid` (`self.GridRenderer`)
    (:`Is Valid`
      (return (`self.GridRenderer`)))
    (:`Is Not Valid`
      (bind _returnvalue (`GameplayStatics.GetActorOfClass` _gridrendererclass))
      (`/Engine/EditorBlueprintResources/StandardMacros.IsValid` _returnvalue
        (:`Is Valid`
          (bind _output_get (set `self.GridRenderer` _returnvalue))
          (return _output_get))
        (:`Is Not Valid`
          (bind _returnvalue_2 (`|SpawnActorFromClass` _gridrendererclass (`KismetMathLibrary.MakeTransform` (0.0 0.0 0.0)) "AlwaysSpawn" "OverrideRootScale" null null))
          (return _returnvalue_2))))))

(fn `GetValidIndices`
  (params (GridManager :type "/Game/Blueprints/Grid/BP_Grid_Manager Object Reference") (IgnoredActors :type "Array of Actor Object Reference"))
  (returns (Result :type "Map of IntPoint Structure to Vector Structure"))
  (locals (ValidIndices :type "Map of IntPoint Structure to Vector Structure"))
  (bind _gridsize (`/Game/Blueprints/Grid/BP_Grid_Manager.GridSize` GridManager))
  (bind _indices (`self.GetCollisionBoxIndices` GridManager))
  (for _array_element _indices
    (bind (_x _y) (break `IntPoint` _array_element))
    (bind _returnvalue (`KismetMathLibrary.MakeVector` (* _x _gridsize) (* _y _gridsize)))
    (bind (_outhit _returnvalue_2) (`KismetSystemLibrary.LineTraceSingle` (+ _returnvalue (`KismetMathLibrary.MakeVector` 0.0 0.0 _gridsize)) (- _returnvalue (`KismetMathLibrary.MakeVector` 0.0 0.0 _gridsize)) "TraceTypeQuery1" false IgnoredActors "ForDuration"))
    (if _returnvalue_2
      (`BlueprintMapLibrary.Map_Add` (`local.ValidIndices`) _array_element (`.Location` (`GameplayStatics.BreakHitResult` _outhit)))))
  (return (`local.ValidIndices`)))

(fn `UserConstructionScript`
  (locals (GridManager :type "/Game/Blueprints/Grid/BP_Grid_Manager Object Reference") (IgnoredPawns :type "Array of Pawn Object Reference")))
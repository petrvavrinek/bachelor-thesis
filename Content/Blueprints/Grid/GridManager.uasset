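; GridManager builds a square grid of walkable points over its nav volumes and renders it as instanced static meshes.
; It traces down through each volume at GridSize steps, ignoring pawns, storing hit locations by integer coordinate and adding a mesh at each.
; Coordinates are relative to each volume's center, so multiple volumes overwrite shared keys.
; The grid rebuilds on BeginPlay or via a construction-script Reset toggle, and helpers provide validity, location and nearest-index lookups.
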(event `self.ReceiveBeginPlay`
  (`self.CalculatePositionsAndRenderMeshes`))

(fn `CalculatePositionsAndRenderMeshes`
  (locals (Origin :type "Vector Structure") (Pawns :type "Array of Pawn Object Reference"))
  (bind _gridsize (`self.GridSize`))
  (bind _gridsize_2 (`self.GridSize`))
  (`InstancedStaticMeshComponent.ClearInstances` (`self.InstancedStaticMesh`))
  (`BlueprintMapLibrary.Map_Clear` (`self.GridIndices`))
  (bind _outactors (`GameplayStatics.GetAllActorsOfClass` "/Script/Engine.Pawn"))
  (set `local.Pawns` _outactors)
  (for _array_element (`self.NavVolumes`)
    (bind (_origin _boxextent) (`self.GetActorBounds` _array_element false false))
    (set `local.Origin` _origin)
    (bind _z (.z _boxextent))
    (bind _returnvalue (`KismetMathLibrary.FFloor` (/ (.x _boxextent) _gridsize)))
    (`KismetSystemLibrary.PrintString` (`KismetStringLibrary.Conv_IntToString` _returnvalue))
    (for _index (range (* _returnvalue -1) (+ _returnvalue 1))
      (bind _returnvalue_2 (`KismetMathLibrary.FFloor` (/ (.y _boxextent) _gridsize)))
      (for _index_2 (range (* _returnvalue_2 -1) (+ _returnvalue_2 1))
        (bind _returnvalue_3 (+ (`local.Origin`) (`KismetMathLibrary.MakeVector` (* _index _gridsize_2) (* _index_2 _gridsize_2) _z)))
        (bind (_outhit _returnvalue_4) (`KismetSystemLibrary.LineTraceSingle` _returnvalue_3 (- _returnvalue_3 (`KismetMathLibrary.MakeVector` 0.0 0.0 (* _z 2.0))) "TraceTypeQuery1" false (`local.Pawns`)))
        (if _returnvalue_4
          (bind (_bblockinghit _binitialoverlap _time _distance _location) (`GameplayStatics.BreakHitResult` _outhit))
          (`BlueprintMapLibrary.Map_Add` (`self.GridIndices`) (make `IntPoint` _index _index_2) _location)
          (`InstancedStaticMeshComponent.AddInstance` (`self.InstancedStaticMesh`) (`KismetMathLibrary.MakeTransform` (+ _location (`self.HitOffset`)) (struct) (`self.PlaneScale`)) true))))))

(fn `GetClosestIndex`
  (params (Index :type "Vector Structure"))
  (returns (OutputPin :type "IntPoint Structure"))
  (locals (Closest :type "IntPoint Structure") (ClosestDistance :type "Float (double-precision)" :default 999999999.0))
  (bind _gridindices (`self.GridIndices`))
  (bind _keys (`BlueprintMapLibrary.Map_Keys` _gridindices))
  (for _array_element _keys
    (bind (_value _returnvalue) (`BlueprintMapLibrary.Map_Find` _gridindices _array_element))
    (if _returnvalue
      (bind _returnvalue_2 (`KismetMathLibrary.Vector_Distance` _value Index))
      (if (< _returnvalue_2 (`local.ClosestDistance`))
        (set `local.ClosestDistance` _returnvalue_2)
        (set `local.Closest` _array_element))))
  (return (`local.Closest`)))

(fn `GetIndexLocation`
  (params (Index :type "IntPoint Structure"))
  (returns (Location :type "Vector Structure") (Found :type Boolean))
  (bind (_value _returnvalue) (`BlueprintMapLibrary.Map_Find` (`self.GridIndices`) Index))
  (return _value _returnvalue))

(fn `IsIndexValid`
  (params (Index :type "IntPoint Structure"))
  (returns (NewParam :type Boolean))
  (return (`BlueprintMapLibrary.Map_Contains` (`self.GridIndices`) Index)))

(fn `UserConstructionScript`
  (locals (Origin :type "Vector Structure" :default (0.0 0.0 0.0)))
  ;[1 1 1] Reset function
  (if (`self.Reset`)
    (set `self.Reset` false)
    (`self.CalculatePositionsAndRenderMeshes`)))
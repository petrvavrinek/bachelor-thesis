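; Player controller for the main menu that sets up the menu UI and its background camera view.
; On BeginPlay it shows the cursor, creates WBP_Game_MainMenu, switches to UI-only input focused on that widget and adds it to the viewport.
; It then looks up the first BP_RotatingAround_Camera in the level and, if valid, makes it the view target.
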(event `self.ReceiveBeginPlay`
  ;[1 1 1] Only create main menu UI
  (set `self.bShowMouseCursor` true)
  (bind _returnvalue (`|CreateWidget` "/Game/Widgets/Game/MainMenu/WBP_Game_MainMenu.WBP_Game_MainMenu_C" self))
  (`WidgetBlueprintLibrary.SetInputMode_UIOnlyEx` self _returnvalue)
  (`UserWidget.AddToViewport` _returnvalue 0)
  (bind _outactors (`GameplayStatics.GetAllActorsOfClass` "/Game/Blueprints/Pawns/BP_RotatingAround_Camera.BP_RotatingAround_Camera_C"))
  (bind _output (`|GetArrayItem` _outactors))
  (`/Engine/EditorBlueprintResources/StandardMacros.IsValid` _output
    (:`Is Valid`
      (`self.SetViewTargetWithBlend` _output))))

(fn `UserConstructionScript`)
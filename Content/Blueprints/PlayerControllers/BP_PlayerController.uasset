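; Player controller that sets up the robot instruction UI at the start of play.
; BeginPlay builds an InstructionBuffer and fills its queue with objects constructed from the AvailableInstructions classes.
; It creates the WBP_GameUI widget with that buffer and the first BP_PlayerRobot found, then adds it to the viewport.
; It shows the mouse cursor and switches to game-and-UI input focused on the widget.
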(event `self.ReceiveBeginPlay`
  (bind _returnvalue (`|GenericCreateObject` "/Game/Blueprints/Instructions/Base/InstructionBuffer.InstructionBuffer_C"))
  (set `self.InstructionBuffer` _returnvalue)
  (for _array_element (`self.AvailableInstructions`)
    (bind _returnvalue_2 (`|GenericCreateObject` _array_element))
    (`KismetArrayLibrary.Array_Add` (`/Game/Blueprints/Instructions/Base/InstructionBuffer.InstructionQueue` (`self.InstructionBuffer`)) _returnvalue_2))
  (bind _outactors (`GameplayStatics.GetAllActorsOfClass` "/Game/Blueprints/Pawns/BP_PlayerRobot.BP_PlayerRobot_C"))
  (bind _returnvalue_3 (`|CreateWidget` "/Game/Widgets/Game/WBP_GameUI.WBP_GameUI_C" self (`self.InstructionBuffer`) (`|GetArrayItem` _outactors)))
  (`UserWidget.AddToViewport` _returnvalue_3 0)
  (set `self.bShowMouseCursor` true)
  (`WidgetBlueprintLibrary.SetInputMode_GameAndUIEx` self _returnvalue_3 "DoNotLock" false))

(fn `UserConstructionScript`)
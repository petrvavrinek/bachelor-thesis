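; Player controller for a robot programming game, where the player runs instructions on a controlled pawn.
; On initialization it builds a root instruction buffer and a palette buffer of allowed instruction instances, then hands both to the in-game tools widget.
; The widget's start event resets the robot's transform and runs the instruction through a new executor and call stack.
; Stop interrupts that executor, and completion with an exception opens an error modal.
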(event `InitializePlayerController`
  (params (AllowedInstructions :type "Array of /Game/Blueprints/Instructions/Instruction Class Reference") (ControlledPawn :type "Pawn Object Reference") (AllowCustomFunctions :type Boolean))
  ;[1 1 1] Handle PC initialization
  (set `self.ControlledPawn` ControlledPawn)
  (bind _returnvalue (`|GenericCreateObject` "/Game/Blueprints/Instructions/InstructionBuffer.InstructionBuffer_C"))
  (set `self.RootInstructionBuffer` _returnvalue)
  (bind _returnvalue_2 (`|GenericCreateObject` "/Game/Blueprints/Instructions/InstructionBuffer.InstructionBuffer_C"))
  (set `self.AvailableInstructionBuffer` _returnvalue_2)
  (for _array_element AllowedInstructions
    (bind _returnvalue_3 (`|GenericCreateObject` _array_element))
    (`KismetArrayLibrary.Array_Add` (`/Game/Blueprints/Instructions/InstructionBuffer.InstructionQueue` (`self.AvailableInstructionBuffer`)) _returnvalue_3))
  (`self.CreateUI` ControlledPawn AllowCustomFunctions))

(event `CreateUI`
  (params (ControlledPawn :type "Pawn Object Reference") (AllowCustomFunctions :type Boolean))
  (bind _returnvalue (`|CreateWidget` "/Game/Widgets/Game/InGame/Tools/WBP_InGame_Tools.WBP_InGame_Tools_C" self))
  (`/Game/Widgets/Game/InGame/Tools/WBP_InGame_Tools.Initialize` _returnvalue (`self.AvailableInstructionBuffer`) (`self.RootInstructionBuffer`) ControlledPawn AllowCustomFunctions)
  (`UserWidget.AddToViewport` _returnvalue 0)
  (set `self.ToolsWidget` _returnvalue)
  (set `self.bShowMouseCursor` true)
  (`WidgetBlueprintLibrary.SetInputMode_GameAndUIEx` self _returnvalue "DoNotLock" false)
  (add `/Game/Widgets/Game/InGame/Tools/WBP_InGame_Tools.OnInstructionStart` _returnvalue (`|CreateDelegate` :!event `OnInstructionStartRequest`))
  (add `/Game/Widgets/Game/InGame/Tools/WBP_InGame_Tools.OnInstructionStop` _returnvalue (`|CreateDelegate` :!event `OnInstructionInterruptRequest`)))

(event `OnInstructionStartRequest`
  (params (Instruction :type "/Game/Blueprints/Instructions/Instruction Object Reference"))
  ;[1 1 1] Handle instruction start
  (bind _asbp_player_robot (cast `/Game/Blueprints/Pawns/BP_PlayerRobot` (`self.ControlledPawn`)))
  (`/Game/Blueprints/Pawns/BP_PlayerRobot.ResetTransform` _asbp_player_robot)
  (bind _returnvalue (`|GenericCreateObject` "/Game/Blueprints/Instructions/InstructionStack.InstructionStack_C"))
  (bind _returnvalue_2 (`|GenericCreateObject` "/Game/Blueprints/Instructions/InstructionExecutor.InstructionExecutor_C" _returnvalue Instruction))
  (bind _output_get (set `self.CurrentExecutor` _returnvalue_2))
  (`/Game/Blueprints/Instructions/Instruction.StartJob` Instruction (`self.ControlledPawn`) _output_get)
  (add `/Game/Blueprints/Instructions/Instruction.OnCompleted` Instruction (`|CreateDelegate` :!event `OnInstructionsComplete`)))

(event `OnInstructionInterruptRequest`
  (params (Instruction :type "/Game/Blueprints/Instructions/Instruction Object Reference"))
  ;[1 1 1] Handle instruction interrupt
  (`/Game/Blueprints/Instructions/InstructionExecutor.Interrupt` (`self.CurrentExecutor`)))

(event `OnInstructionsComplete`
  (params (Exception :type "/Game/Blueprints/Instructions/InstructionException Object Reference") (Executor :type "/Game/Blueprints/Instructions/InstructionExecutor Object Reference") (ControlledPawn :type "Pawn Object Reference"))
  ;[1 1 1] Handle instruction complete
  (`/Engine/EditorBlueprintResources/StandardMacros.IsValid` Exception
    (:`Is Valid`
      (bind _returnvalue (`|CreateWidget` "/Game/Widgets/Game/InGame/Components/WBP_InstructionErrorModal.WBP_InstructionErrorModal_C" self Exception))
      (bind _returnvalue_2 (`/Game/Blueprints/Functions/GameFunctions.CreateModalWindow` _returnvalue true))
      (`UserWidget.AddToViewport` _returnvalue_2 0))))

(fn `UserConstructionScript`)
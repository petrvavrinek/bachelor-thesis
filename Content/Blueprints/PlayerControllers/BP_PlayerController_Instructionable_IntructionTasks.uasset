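; Player controller for task-based instruction levels, extending its parent's UI with a task list that tracks completion.
; On UI creation, it builds the tasks widget from the game mode's InstructionGameDescriptor_Task and shows it in place of the tools widget.
; The M key flip-flops between tools and tasks widgets.
; When instructions complete without a valid exception, it shows the tasks widget and updates each task's completion status.
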(event `self.CreateUI`
  (params (ControlledPawn :type "Pawn Object Reference") (AllowCustomFunctions :type Boolean))
  (`parent.CreateUI` ControlledPawn AllowCustomFunctions)
  (bind _asbp_game_mode_game_descriptor (cast `/Game/Blueprints/GameModes/BP_GameMode_GameDescriptor` (`GameplayStatics.GetGameMode`))
    (:`then`
      (bind _asinstruction_game_descriptor_task (cast `/Game/Blueprints/GameDescriptors/InstructionGameDescriptor_Task` (`/Game/Blueprints/GameModes/BP_GameMode_GameDescriptor.GameDescriptor` _asbp_game_mode_game_descriptor))
        (:`then`
          (`Widget.RemoveFromParent` (`self.ToolsWidget`))
          (bind _returnvalue (`|CreateWidget` "/Game/Widgets/Game/InGame/Tasks/WBP_InGame_InstructionTasks.WBP_InGame_InstructionTasks_C" null (`/Game/Blueprints/GameDescriptors/InstructionGameDescriptor_Task.Tasks` _asinstruction_game_descriptor_task)))
          (`UserWidget.AddToViewport` _returnvalue 0)
          (set `self.InstructionTasksWidget` _returnvalue))
        (:`CastFailed`
          (`GameUtils.PrintDebugString` "Game Descriptor in BP_GameMode_Descriptor is not child of InstructionGameDescriptor_Task" (struct :`R` 0.5 :`G` 0.159568 :`A` 1.0) 3.0))))
    (:`CastFailed`
      (`GameUtils.PrintDebugString` "Current GameMode is not BP_GameMode_Descriptor" (struct :`R` 0.5 :`G` 0.159568 :`A` 1.0) 3.0))))

(event `ShowToolsWidget`
  (`Widget.RemoveFromParent` (`self.InstructionTasksWidget`))
  (`UserWidget.AddToViewport` (`self.ToolsWidget`) 0))

(event `Key|M`
  (params (Key :type "Key Structure"))
  (:`Pressed`
    (`/Engine/EditorBlueprintResources/StandardMacros.FlipFlop`
      (:`A`
        (`self.ShowToolsWidget`))
      (:`B`
        (`self.ShowTasksWidget`)))))

(event `ShowTasksWidget`
  (`Widget.RemoveFromParent` (`self.ToolsWidget`))
  (`UserWidget.AddToViewport` (`self.InstructionTasksWidget`) 0))

(event `self.OnInstructionsComplete`
  (params (Exception :type "/Game/Blueprints/Instructions/InstructionException Object Reference") (Executor :type "/Game/Blueprints/Instructions/InstructionExecutor Object Reference") (ControlledPawn :type "Pawn Object Reference"))
  (`parent.OnInstructionsComplete` Exception Executor ControlledPawn)
  (`/Engine/EditorBlueprintResources/StandardMacros.IsValid` Exception
    (:`Is Not Valid`
      (`self.ShowTasksWidget`)
      (bind _asbp_game_mode_game_descriptor (cast `/Game/Blueprints/GameModes/BP_GameMode_GameDescriptor` (`GameplayStatics.GetGameMode`)))
      (bind _asinstruction_game_descriptor_task (cast `/Game/Blueprints/GameDescriptors/InstructionGameDescriptor_Task` (`/Game/Blueprints/GameModes/BP_GameMode_GameDescriptor.GameDescriptor` _asbp_game_mode_game_descriptor)))
      (for _array_element (`/Game/Blueprints/GameDescriptors/InstructionGameDescriptor_Task.Tasks` _asinstruction_game_descriptor_task)
        (bind _completed (`/Game/Blueprints/InstructionTasks/InstructionTask.IsCompleted` _array_element (`self.RootInstructionBuffer`) (`self.ControlledPawn`) Executor Exception))
        (`/Game/Widgets/Game/InGame/Tasks/WBP_InGame_InstructionTasks.SetInstructionCompletionStatus` (`self.InstructionTasksWidget`) _array_element _completed)))))

(fn `UserConstructionScript`
  (`parent.UserConstructionScript`))
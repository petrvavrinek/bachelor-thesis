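; Game mode for task-based instruction that supplies a game descriptor populated with the tasks provided by actors in the world.
; Its GetGameDescriptor override casts the parent's descriptor to InstructionGameDescriptor_Task, then appends tasks gathered from every BI_InstructionTask_Actor implementer.
; Tasks are added on each call without clearing the list, and each addition is printed.
; A failed cast prints a debug message and returns the parent descriptor unchanged.
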(fn `GetGameDescriptor`
  (returns (GameDescriptor :type "/Game/Blueprints/GameDescriptors/InstructionGameDescriptor Object Reference"))
  (bind _gamedescriptor (`parent.GetGameDescriptor`))
  (bind _asinstruction_game_descriptor_task (cast `/Game/Blueprints/GameDescriptors/InstructionGameDescriptor_Task` _gamedescriptor)
    (:`then`
      (bind _outactors (`GameplayStatics.GetAllActorsWithInterface` "/Game/Blueprints/InstructionTasks/BI_InstructionTask_Actor.BI_InstructionTask_Actor_C"))
      (for _array_element _outactors
        (bind _instructiontasks (message `/Game/Blueprints/InstructionTasks/BI_InstructionTask_Actor.GetInstructionTasks` _array_element))
        (for _array_element_2 _instructiontasks
          (`KismetArrayLibrary.Array_Add` (`/Game/Blueprints/GameDescriptors/InstructionGameDescriptor_Task.Tasks` _asinstruction_game_descriptor_task) _array_element_2)
          (`KismetSystemLibrary.PrintText` (`|FormatText` "added {0} to {1}" (`KismetSystemLibrary.GetObjectName` _array_element_2) (`KismetSystemLibrary.GetObjectName` _gamedescriptor)) false)))
      (return _asinstruction_game_descriptor_task))
    (:`CastFailed`
      (`GameUtils.PrintDebugString` (`KismetTextLibrary.Conv_TextToString` (`|FormatText` "{0} is not base of InstructionGameDescriptor_Task" (`KismetSystemLibrary.GetObjectName` _gamedescriptor))))
      (return _gamedescriptor))))

(fn `UserConstructionScript`)
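; Game mode that sets up an instruction-driven level from a game descriptor taken from the game instance, with a local or newly constructed fallback.
; On BeginPlay it spawns the descriptor's pawn at the first TargetPoint with a default controller.
; It passes the pawn and allowed instructions to BP_PlayerController_Instructionable.
; The player possesses a separate BP_PlayerRotateAround_Robot pawn attached to the spawned pawn.
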(event `self.ReceiveBeginPlay`
  (bind _returnvalue (`GameplayStatics.GetPlayerController` 0))
  (bind _gamedescriptor (`self.GameDescriptor`))
  (bind _gamedescriptor_2 (`self.GetGameDescriptor`))
  (set `self.GameDescriptor` _gamedescriptor_2)
  (bind _outactors (`GameplayStatics.GetAllActorsOfClass` "/Script/Engine.TargetPoint"))
  (bind (_returnvalue_location _returnvalue_rotation) (`KismetMathLibrary.BreakTransform` (`self.GetTransform` (`|GetArrayItem` _outactors))))
  (bind _returnvalue_2 (`|SpawnActorFromClass` (`/Game/Blueprints/GameDescriptors/InstructionGameDescriptor.Pawn` (`self.GameDescriptor`)) (`KismetMathLibrary.MakeTransform` _returnvalue_location _returnvalue_rotation) "AlwaysSpawn" "OverrideRootScale" (`GameplayStatics.GetPlayerController` 0) null))
  (`Pawn.SpawnDefaultController` _returnvalue_2)
  (bind _asbp_player_controller_instructionable (cast `/Game/Blueprints/PlayerControllers/BP_PlayerController_Instructionable` (`GameplayStatics.GetPlayerController` 0)))
  (`/Game/Blueprints/PlayerControllers/BP_PlayerController_Instructionable.InitializePlayerController` _asbp_player_controller_instructionable (`/Game/Blueprints/GameDescriptors/InstructionGameDescriptor.AvailableInstructions` _gamedescriptor) _returnvalue_2 (`/Game/Blueprints/GameDescriptors/InstructionGameDescriptor.AllowCustomFunctions` _gamedescriptor))
  (bind _returnvalue_3 (`|SpawnActorFromClass` "/Game/Blueprints/Pawns/BP_PlayerRotateAround_Robot.BP_PlayerRotateAround_Robot_C" (`KismetMathLibrary.Conv_VectorToTransform` (`self.K2_GetActorLocation` _returnvalue_2)) "AlwaysSpawn" "OverrideRootScale" _returnvalue null))
  (`Controller.Possess` _returnvalue _returnvalue_3)
  (`/Game/Blueprints/Pawns/BP_PlayerRotateAround_Robot.SetAttachToPawn` _returnvalue_3 _returnvalue_2))

(fn `GetGameDescriptor`
  (returns (GameDescriptor :type "/Game/Blueprints/GameDescriptors/InstructionGameDescriptor Object Reference"))
  (bind _gamedescriptor (`self.GameDescriptor`))
  (bind _asbp_game_instance (cast `/Game/Blueprints/BP_GameInstance` (`GameplayStatics.GetGameInstance`))
    (:`then`
      (bind _gamedescriptor_2 (`/Game/Blueprints/BP_GameInstance.GameDescriptor` _asbp_game_instance))
      (`/Engine/EditorBlueprintResources/StandardMacros.IsValid` _gamedescriptor_2
        (:`Is Valid`
          (return _gamedescriptor_2))
        (:`Is Not Valid`
          _)))
    (:`CastFailed`
      _))
  (`/Engine/EditorBlueprintResources/StandardMacros.IsValid` _gamedescriptor
    (:`Is Valid`
      (return _gamedescriptor))
    (:`Is Not Valid`
      (bind _returnvalue (`|GenericCreateObject` (`self.GameDescriptorClass`)))
      (`/Game/Blueprints/GameDescriptors/InstructionGameDescriptor.OnInitialize` _returnvalue)
      (return _returnvalue))))

(fn `UserConstructionScript`)
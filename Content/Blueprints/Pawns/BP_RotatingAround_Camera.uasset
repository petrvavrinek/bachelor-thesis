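; BP_RotatingAround_Camera is an orbiting camera that rotates around a target actor.
; The construction script moves it to a valid TargetActor, sets the spring arm length from Distance, and aims the camera using a look-at rotation flipped 180 degrees.
; Each tick it yaws the Scene component by RotationSpeed scaled by delta time, without updating the target's position.
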(event `self.ReceiveTick`
  (params (DeltaSeconds :type "Float (single-precision)"))
  (`SceneComponent.K2_AddLocalRotation` (`self.Scene`) (`KismetMathLibrary.MakeRotator` 0.0 0.0 (* DeltaSeconds (`self.RotationSpeed`))) false false))

(fn `UserConstructionScript`
  (bind _targetactor (`self.TargetActor`))
  (bind _returnvalue (`self.K2_GetActorLocation` _targetactor))
  (`/Engine/EditorBlueprintResources/StandardMacros.IsValid` _targetactor
    (:`Is Valid`
      (`self.K2_SetActorLocation` _returnvalue)
      (set `SpringArmComponent.TargetArmLength` (`self.Distance`) (`self.SpringArm`))
      (`SceneComponent.K2_SetWorldRotation` (`self.Camera`) (`KismetMathLibrary.ComposeRotators` (`KismetMathLibrary.FindLookAtRotation` _returnvalue (`SceneComponent.K2_GetComponentLocation` (`self.Camera`))) (struct :`Yaw` -180.0)) false false))))
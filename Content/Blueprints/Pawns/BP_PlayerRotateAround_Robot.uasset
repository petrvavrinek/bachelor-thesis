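; Orbit camera pawn, named for the robot, that follows an assigned target and lets the player rotate and zoom around it.
; SetAttachToPawn stores the target, and Tick moves the root to its location each frame without a true attachment, so only position is copied.
; Mouse axes yaw the spring arm and pitch it within a clamped downward-looking range, while the wheel adjusts arm length within fixed limits.
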(event `InputAxisKey|MouseX`
  (params (AxisValue :type "Float (single-precision)"))
  (`SceneComponent.K2_AddRelativeRotation` (`self.SpringArm`) (`KismetMathLibrary.MakeRotator` 0.0 0.0 AxisValue) false false))

(event `InputAxisKey|MouseY`
  (params (AxisValue :type "Float (single-precision)"))
  (bind _springarm (`self.SpringArm`))
  (bind (_relativerotation_roll _relativerotation_pitch _relativerotation_yaw) (`KismetMathLibrary.BreakRotator` (`SceneComponent.RelativeRotation` _springarm)))
  (`SceneComponent.K2_SetRelativeRotation` _springarm (`KismetMathLibrary.MakeRotator` 0.0 (`KismetMathLibrary.FClamp` (+ AxisValue _relativerotation_pitch) -89.0 0.0) _relativerotation_yaw) false false))

(event `self.ReceiveTick`
  (params (DeltaSeconds :type "Float (single-precision)"))
  (bind _attachtoactor (`self.AttachToActor`))
  (`/Engine/EditorBlueprintResources/StandardMacros.IsValid` _attachtoactor
    (:`Is Valid`
      (`SceneComponent.K2_SetWorldLocation` (`self.DefaultSceneRoot`) (`self.K2_GetActorLocation` _attachtoactor) false false))))

(event `SetAttachToPawn`
  (params (Pawn :type "Pawn Object Reference"))
  (set `self.AttachToActor` Pawn))

(event `InputAxisKey|MouseWheelAxis`
  (params (AxisValue :type "Float (single-precision)"))
  (set `SpringArmComponent.TargetArmLength` (`KismetMathLibrary.FClamp` (+ (* AxisValue -20.0) (`SpringArmComponent.TargetArmLength` (`self.SpringArm`))) 300.0 800.0) (`self.SpringArm`)))

(fn `UserConstructionScript`)
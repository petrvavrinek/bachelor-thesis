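; Player robot pawn that executes turn-left and move-forward instructions on a grid, reporting each one as completed.
; Turns animate yaw through a timeline from the starting rotation.
; Forward moves target the facing neighbor index through GridMovementComponent and complete on its move-done event, regardless of success.
; Spawns its default controller on BeginPlay and draws a debug arrow toward the cell ahead every tick.
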(event `self.ReceiveBeginPlay`
  (`self.SpawnDefaultController`))

(event `TurnLeft`
  (params (Instruction :type "/Game/Blueprints/Instructions/Base/Instruction Object Reference"))
  (bind (_returnvalue_roll _returnvalue_pitch _returnvalue_yaw) (`KismetMathLibrary.BreakRotator` (`self.K2_GetActorRotation`)))
  ;[1 1 1] Rotating
  (set `self.StartRotationZ` _returnvalue_yaw)
  (bind (_direction _rotationz) (`Timeline|TurnLeftTimeline` :!via `PlayFromStart`)
    (:`Update`
      (`self.K2_SetActorRotation` (`KismetMathLibrary.MakeRotator` _returnvalue_roll _returnvalue_pitch (- (`self.StartRotationZ`) _rotationz))))
    (:`Finished`
      (`self.OnInstructionCompleted` Instruction))))

(event `MoveForward`
  (params (Instruction :type "/Game/Blueprints/Instructions/Base/Instruction Object Reference"))
  (bind _gridmovementcomponent (`self.GridMovementComponent`))
  ;[1 1 1] Moving forward
  (set `self.CurrentInstruction` Instruction)
  (add `/Game/Blueprints/Components/BP_GridMovementComponent.OnMoveDone` _gridmovementcomponent (delegate `OnMovementForwardDone`))
  (`/Game/Blueprints/Components/BP_GridMovementComponent.MoveToIndex` _gridmovementcomponent (+ (`/Game/Blueprints/Components/BP_GridMovementComponent.GetDirectionForwardIndex` _gridmovementcomponent) (`/Game/Blueprints/Components/BP_GridMovementComponent.GetCurrentGridIndex` _gridmovementcomponent))))

(event `OnMovementForwardDone`
  (params (success :type Boolean))
  ;[1 1 1] Moving forward
  (remove `/Game/Blueprints/Components/BP_GridMovementComponent.OnMoveDone` (`self.GridMovementComponent`) (delegate `OnMovementForwardDone`))
  (`self.OnInstructionCompleted` (`self.CurrentInstruction`))
  (set `self.CurrentInstruction` null))

(event `self.ReceiveTick`
  (params (DeltaSeconds :type "Float (single-precision)"))
  (bind _gridmovementcomponent (`self.GridMovementComponent`))
  (bind _currentgridpositionindex (`/Game/Blueprints/Components/BP_GridMovementComponent.GetCurrentGridIndex` _gridmovementcomponent))
  (bind _gridmanager (`/Game/Blueprints/Components/BP_GridMovementComponent.GridManager` _gridmovementcomponent))
  (bind (_location _found) (`/Game/Blueprints/Grid/GridManager.GetIndexLocation` _gridmanager _currentgridpositionindex))
  (bind _returnvalue (`KismetMathLibrary.MakeVector` 0.0 0.0 (`CapsuleComponent.GetScaledCapsuleHalfHeight` (`self.CapsuleComponent`))))
  (bind (_location_2 _found_2) (`/Game/Blueprints/Grid/GridManager.GetIndexLocation` _gridmanager (+ (`/Game/Blueprints/Components/BP_GridMovementComponent.GetDirectionForwardIndex` _gridmovementcomponent) _currentgridpositionindex)))
  (if (and _found _found_2)
    (`KismetSystemLibrary.DrawDebugArrow` (+ _location _returnvalue) (+ _location_2 _returnvalue) 80.0 (struct :`R` 1.0 :`G` 0.063568 :`A` 1.0) 0.0 10.0)))

(fn `UserConstructionScript`)
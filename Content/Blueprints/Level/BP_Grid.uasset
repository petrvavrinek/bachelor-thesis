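; BP_Grid is a level actor that builds a flat grid of instanced mesh blocks.
; Its construction script clears the instanced static mesh, then loops over the X and Y block counts, adding one thin, Z-flattened instance per cell.
; Cells are spaced by block size in local space and shifted back by half the total grid size to sit around the actor's origin.
; The event graph has no active logic.
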(fn `UserConstructionScript`
  (locals (TotalSize :type "Vector2D Structure"))
  (bind (_x _y) (`KismetMathLibrary.BreakVector2D` (`self.BlockSize`)))
  (bind (_x_2 _y_2) (break `IntPoint` (- (`self.NumberOfBlocks`) (make `IntPoint` 1 1))))
  (`InstancedStaticMeshComponent.ClearInstances` (`self.InstancedStaticMesh`))
  (set `local.TotalSize` (* (`self.NumberOfBlocks`) (`self.BlockSize`)))
  (for _index (range (+ _x_2 1))
    (for _index_2 (range (+ _y_2 1))
      (`InstancedStaticMeshComponent.AddInstance` (`self.InstancedStaticMesh`) (`KismetMathLibrary.MakeTransform` (- (`KismetMathLibrary.MakeVector` (* _index _x) (* _index_2 _y)) (/ (`local.TotalSize`) (2.0 2.0 2.0))) (struct) (1.0 1.0 0.2)) false))))
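; Actor component that gives a character grid-based movement by tracking its current cell index on a grid manager.
; On BeginPlay it caches the owner's CharacterMovementComponent, optionally auto-finds the manager, takes the closest index and can snap the pawn onto it.
; MoveToIndex uses AI MoveTo to reach a cell, updating the index only on success and reporting the result through CallOnMoveDone.
; A helper rounds the forward vector into an X/Y grid direction.
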(event `self.ReceiveBeginPlay`
  (bind _returnvalue (`Actor.GetComponentByClass` (`self.GetOwner`) "/Script/Engine.CharacterMovementComponent"))
  ;[1 1 1] Begin play
  (`/Engine/EditorBlueprintResources/StandardMacros.IsValid` _returnvalue
    (:`Is Valid`
      (set `self.MovementComponent` _returnvalue)
      (`self.SetCurrentGridManager`)
      (`self.SetCurrentGridIndex`))
    (:`Is Not Valid`
      (`GameUtils.PrintDebugString` "owner pawn does not have CharacterMovement component"))))

(event `SetCurrentGridManager`
  ;[1 1 1] Set initial grid manager
  (if (`self.AutoFindGlobalManager`)
    (bind _output_get (set `self.GridManager` (`/Game/Blueprints/Functions/GridFunctions.GetGridManager`)))
    (`/Engine/EditorBlueprintResources/StandardMacros.IsValid` _output_get
      (:`Is Not Valid`
        (`GameUtils.PrintDebugString` "cannot find grid manager" (struct :`R` 0.5 :`G` 0.118059 :`A` 1.0))))))

(event `SetCurrentGridIndex`
  (bind _gridmanager (`self.GridManager`))
  (bind _returnvalue (`PawnMovementComponent.GetPawnOwner` (`self.MovementComponent`)))
  ;[1 1 1] Set initial position index
  (bind _output_get (set `self.CurrentGridPositionIndex` (`/Game/Blueprints/Grid/BP_Grid_Manager.GetClosestIndex` _gridmanager (`Actor.K2_GetActorLocation` _returnvalue))))
  (if (`self.AlignToGrid`)
    (bind (_location _found) (`/Game/Blueprints/Grid/BP_Grid_Manager.GetIndexLocation` _gridmanager _output_get))
    (if _found
      (`Actor.K2_SetActorLocation` _returnvalue (+ _location (`self.AdditionalLocationPosition`)) true true)
      (else
        (`GameUtils.PrintDebugString` "invalid start index found")))))

(event `MoveToIndex`
  (params (Location :type "IntPoint Structure"))
  (bind (_location _found) (`/Game/Blueprints/Grid/BP_Grid_Manager.GetIndexLocation` (`self.GridManager`) Location))
  ;[1 1 1] Move to index
  (if _found
    (`|AIMoveTo` (`PawnMovementComponent.GetPawnOwner` (`self.MovementComponent`)) _location null 0.001
      (:`OnSuccess`
        (set `self.CurrentGridPositionIndex` Location)
        (`self.OnMoveDone` true))
      (:`OnFail`
        (`self.OnMoveDone` false)))
    (else
      (`self.OnMoveDone` false))))

(fn `GetCurrentGridIndex`
  (returns (CurrentGridPositionIndex :type "IntPoint Structure"))
  (return (`self.CurrentGridPositionIndex`)))

(fn `GetDirectionForwardIndex`
  (returns (DirectionIndex :type "IntPoint Structure"))
  (bind (_returnvalue_x _returnvalue_y) (`KismetMathLibrary.BreakVector` (`Actor.GetActorForwardVector` (`self.GetOwner`))))
  (return (make `IntPoint` (`KismetMathLibrary.Round` _returnvalue_x) (`KismetMathLibrary.Round` _returnvalue_y))))